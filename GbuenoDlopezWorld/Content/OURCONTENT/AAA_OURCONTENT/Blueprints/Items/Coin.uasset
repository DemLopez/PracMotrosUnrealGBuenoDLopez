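; Coin is a pickup item that awards coins to the player's third-person character.
; It sets its coin value to a fixed amount at BeginPlay and inherits the pick-up flow from a parent item class.
; When the pickup ends, it casts the first player's character to ThirdPersonCharacter, adds the coins, then calls the parent's end-pick logic.
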(event EventBeginPlay
  (Variables|Default|SetCoinNum 10))

(event EventTick
  (params (DeltaSeconds :type Float%20%28single-precision%29))
  (|CallParentFunction DeltaSeconds) ; This node is disabled and will not be called.\nDrag off pins to build functionality.
)

(fn ConstructionScript)

(fn MPickItem
  (bind _itempicked (|CallParentFunction))
  (return _itempicked))

(fn MEndPickItem
  (bind _asthird_person_character (Utilities|Casting|CastToThirdPersonCharacter (Game|GetPlayerCharacter 0)))
  (Default|AddCoins _asthird_person_character (Variables|Default|GetCoinNum))
  (|CallParentFunction))