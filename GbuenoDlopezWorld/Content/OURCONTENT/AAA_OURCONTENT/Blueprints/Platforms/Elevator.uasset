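; Elevator platform actor that moves continuously up and down around its starting height.
; BeginPlay stores the starting Z, then Tick moves the actor by MovSpeed scaled by world delta seconds.
; An Up flag flips when the actor passes Goal units above or below the start, so it oscillates across twice that distance.
; The construction script and SetGoalPosition function are empty.
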(event Custom|Move%20Elevator%20UP
  (bind _returnvalue (Transformation|GetActorLocation))
  ;[1 1 1] Up
  (Transformation|SetActorRelativeLocation (Math|Vector|MakeVector (.x _returnvalue) (.y _returnvalue) (+ (.z _returnvalue) (* (Utilities|Time|GetWorldDeltaSeconds) (Variables|Default|GetMovSpeed)))))
  (if (>= (.z (Transformation|GetActorLocation)) (+ (Variables|Default|GetDistance) (Variables|Default|GetGoal)))
    (Variables|Default|SetUp false)))

(event Custom|Move%20Elevator%20Down
  (bind _returnvalue (Transformation|GetActorLocation))
  ;[1 1 1] Down
  (Transformation|SetActorRelativeLocation (Math|Vector|MakeVector (.x _returnvalue) (.y _returnvalue) (- (.z _returnvalue) (* (Utilities|Time|GetWorldDeltaSeconds) (Variables|Default|GetMovSpeed)))))
  (if (<= (.z (Transformation|GetActorLocation)) (- (Variables|Default|GetDistance) (Variables|Default|GetGoal)))
    (Variables|Default|SetUp true)))

(event EventBeginPlay
  (Variables|Default|SetUp true)
  (Variables|Default|SetDistance (.z (Transformation|GetActorLocation))))

(event EventTick
  (params (DeltaSeconds :type Float%20%28single-precision%29))
  (if (Variables|Default|GetUp)
    (CallFunction|MoveElevatorUP)
    (else
      (CallFunction|MoveElevatorDown))))

(fn ConstructionScript)

(fn SetGoalPosition)