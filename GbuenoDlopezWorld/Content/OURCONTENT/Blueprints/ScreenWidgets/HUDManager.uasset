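; HUDManager creates the player HUD widget and keeps its on-screen text in sync with the ItemManager's items.
; SetHUD, which BeginPlay does not call, takes the first ItemManager found in the level, binds to its status changes and adds the widget to the viewport.
; GetPlayerHud lazily creates and caches the widget, though SetHUD also makes a separate, unused one.
; Each status change reprints the item list.
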(event Custom|ItemManagerStatusChanges
  (Default|PrintTextonScreen (Variables|Default|GetPlayerHUD) (Variables|/Game/OURCONTENT/Blueprints/Items/ItemManager.ItemManager_C|GetItems (Variables|Default|GetItemManager))))

(event Custom|Set%20HUD
  (CallFunction|SetItemManager)
  (EventDispatchers|BindEventtoItemManagerStatus (Variables|Default|GetItemManager) (delegate Custom|ItemManagerStatusChanges))
  (UserInterface|CreateWidget "/Game/OURCONTENT/Blueprints/ScreenWidgets/PlayerHUD.PlayerHUD_C")
  (UserInterface|Viewport|AddtoViewport (CallFunction|GetPlayerHud) 0)
  (Default|PrintTextonScreen (Variables|Default|GetPlayerHUD) (Variables|/Game/OURCONTENT/Blueprints/Items/ItemManager.ItemManager_C|GetItems (Variables|Default|GetItemManager)))
  (Development|PrintString "Hello"))

(event EventBeginPlay)

(fn ConstructionScript)

(fn SetItemManager
  (bind _outactors (Actor|GetAllActorsOfClass "/Game/OURCONTENT/Blueprints/Items/ItemManager.ItemManager_C"))
  (Variables|Default|SetItemManager (Utilities|Array|Get(acopy) _outactors)))

(fn GetPlayerHud
  (Variables|Default|GetPlayerHUD
    (:then
      _)
    (:else
      (bind _returnvalue (UserInterface|CreateWidget "/Game/OURCONTENT/Blueprints/ScreenWidgets/PlayerHUD.PlayerHUD_C"))
      (Variables|Default|SetPlayerHUD _returnvalue)))
  (return (Variables|Default|GetPlayerHUD)))