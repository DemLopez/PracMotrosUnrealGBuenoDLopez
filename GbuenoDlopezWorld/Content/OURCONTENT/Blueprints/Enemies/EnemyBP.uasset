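; Enemy character Blueprint with health, an HP bar widget, ragdoll death and run animation.
; Tick polls health and velocity, setting Running on EnemyAnimationBP and switching the mesh to ragdoll physics without capsule collision at zero health.
; TakeDamage updates health and its percentage, while BeginPlay hands the EnemyHPBar widget a self reference.
; PlayerPosses lets player controller 0 possess the enemy and enables input.
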(event EventBeginPlay
  (Variables|Default|SetDEAD? false)
  (bind _output_get (Variables|Default|SetMaxHealth 1e+02))
  (Variables|Default|SetCurrentHealth _output_get)
  (CallFunction|SetHPBar))

(event EventTick
  (params (DeltaSeconds :type Float%20%28single-precision%29))
  (CallFunction|CheckHP)
  (CallFunction|CheckRUN))

(fn ConstructionScript)

(fn CheckHP
  (if (or (Variables|Default|GetDEAD?) (<= (Variables|Default|GetCurrentHealth) 0.0))
    (Variables|Default|SetAIControllerClass 0)
    (Collision|SetCollisionProfileName (Variables|Character|GetMesh) "Ragdoll" :!class /Script/Engine.PrimitiveComponent)
    (Physics|SetSimulatePhysics (Variables|Character|GetMesh) true)
    (Collision|SetCollisionEnabled (Variables|Collision|GetCapsuleComponent) "NoCollision")))

(fn CheckRUN
  (bind _returnvalue (Transformation|GetVelocity))
  (bind _mesh (Variables|Character|GetMesh))
  (bind _returnvalue_2 (Components|SkeletalMesh|GetAnimInstance _mesh))
  (if (or (!= (.x _returnvalue) 0.0) (!= (.y _returnvalue) 0.0))
    (bind _asenemy_animation_bp (Utilities|Casting|CastToEnemyAnimationBP _returnvalue_2))
    (Variables|/Game/OURCONTENT/Blueprints/Enemies/EnemyAnimationBP.EnemyAnimationBP_C|SetRunning _asenemy_animation_bp true)
    (else
      (bind _asenemy_animation_bp_2 (Utilities|Casting|CastToEnemyAnimationBP _returnvalue_2))
      (Variables|/Game/OURCONTENT/Blueprints/Enemies/EnemyAnimationBP.EnemyAnimationBP_C|SetRunning _asenemy_animation_bp_2 false))))

(fn TakeDamage
  (params (Damage :type Float%20%28single-precision%29))
  (bind _output_get (Variables|Default|SetCurrentHealth (- (Variables|Default|GetCurrentHealth) Damage)))
  (Variables|Default|SetHealthPercentage (/ _output_get (Variables|Default|GetMaxHealth))))

(fn SetHPBar
  (Variables|Default|SetHealthPercentage (/ (Variables|Default|GetCurrentHealth) (Variables|Default|GetMaxHealth)))
  (bind _asenemy_hpbar (Utilities|Casting|CastToEnemyHPBar (UserInterface|GetUserWidgetObject (Variables|Default|GetHP%20Bar))))
  (Variables|/Game/OURCONTENT/Blueprints/ScreenWidgets/EnemyHPBar.EnemyHPBar_C|SetEnemies _asenemy_hpbar self))

(fn PlayerPosses
  (bind _returnvalue (Game|GetPlayerController 0))
  (bind _self self)
  (Pawn|Possess _returnvalue _self)
  (Input|EnableInput _self _returnvalue)
  (Development|PrintString "Hello"))