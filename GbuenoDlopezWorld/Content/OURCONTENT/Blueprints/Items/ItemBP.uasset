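; ItemBP is a collectible item Actor that reports its type when picked and removes itself once collection ends.
; PickItem wraps MPickItem, which prints the ItemType enum value and returns it to the caller.
; The EndPick event calls MEndPickItem, which prints a collected message and destroys the actor, so pickup is split into a query step and a removal step.
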(event EventBeginPlay)

(event EventTick
  (params (DeltaSeconds :type Float%20%28single-precision%29)))

(event EventEndPick
  (CallFunction|MEndPickItem))

(fn ConstructionScript)

(fn MPickItem
  (bind _itemtype (Variables|Default|GetItemType))
  (Development|PrintString (Utilities|String|EnumtoString _itemtype))
  (return _itemtype))

(fn MEndPickItem
  (Development|PrintString "Item Collected")
  (Actor|DestroyActor))

(fn PickItem
  (bind _itempicked (CallFunction|MPickItem))
  (return _itempicked))