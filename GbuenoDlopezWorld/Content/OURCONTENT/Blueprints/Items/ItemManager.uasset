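; ItemManager is a Blueprint that keeps count of the keys and coins picked up in the game.
; ItemPicked switches on the item type and increments the matching "Keys" or "Coins" entry in the Items map.
; It then fires the ItemManagerStatus dispatcher, without passing arguments, to signal the update to any bound listeners.
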(fn ConstructionScript)

(fn ItemPicked
  (params (Item :type ItemENUM%20Enum :default "NewEnumerator0"))
  (Utilities|FlowControl|Sequence
    (:then_0
      (switch Utilities|FlowControl|Switch|SwitchonItemENUM Item
        (:NewEnumerator0
          (bind _result (Math|Integer|IncrementInt (.Value (Utilities|Map|Find (Variables|Default|GetItems) "Keys")))
            (:%20%20
              (Utilities|Map|Add (Variables|Default|GetItems) "Keys" _result))))
        (:NewEnumerator1
          (bind _result_2 (Math|Integer|IncrementInt (.Value (Utilities|Map|Find (Variables|Default|GetItems) "Coins")))
            (:%20%20
              (Utilities|Map|Add (Variables|Default|GetItems) "Coins" _result_2))))))
    (:then_1
      (Default|CallItemManagerStatus))))