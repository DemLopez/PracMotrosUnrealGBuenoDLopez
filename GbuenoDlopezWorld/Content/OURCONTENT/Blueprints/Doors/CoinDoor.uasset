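; CoinDoor is a child door Blueprint gated by the player's coin count.
; On BeginPlay it builds its requirement text from RequiredCoins, displayed divided by ten.
; When a Player-tagged FPS_Character overlaps, it compares Coins against the undivided RequiredCoins and calls the parent overlap logic only if there are enough.
; Otherwise it prints a not-enough-coins message, and no coins are deducted here.
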(event EventBeginPlay
  (|CallParentFunction)
  (Variables|Default|SetRequirementText (Utilities|String|Append "You need " (Utilities|String|ToString(Integer) (/ (Variables|Default|GetRequiredCoins) 10)) " Coins"))
  (CallFunction|SetRequirementText))

(event Collision|EventActorBeginOverlap
  (params (OtherActor :type Actor%20Object%20Reference))
  (if (Actor|ActorHasTag OtherActor "Player")
    (bind _asfps_character (Utilities|Casting|CastToFPS_Character OtherActor))
    (if (>= (Variables|/Game/OURCONTENT/FPS/Character/FPS_Character.FPS_Character_C|GetCoins _asfps_character) (Variables|Default|GetRequiredCoins))
      (|CallParentFunction OtherActor)
      (else
        (Development|PrintString "You Dont have Enough Coins !")))))

(event EventTick
  (params (DeltaSeconds :type Float%20%28single-precision%29))
  (|CallParentFunction DeltaSeconds))

(fn ConstructionScript
  (|CallParentFunction))