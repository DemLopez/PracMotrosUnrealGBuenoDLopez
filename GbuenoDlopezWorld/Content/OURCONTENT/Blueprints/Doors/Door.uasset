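; Door actor that swings open when a Player-tagged actor overlaps it and closes once the player moves away.
; BeginPlay marks it closed and shows its requirement text on DoorReq, though opening checks no requirement.
; Opening snaps the actor 90 degrees in yaw and clears that text, which closing never restores.
; While open, Tick compares player distance to a threshold and reverses the rotation when exceeded.
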(event Custom|Open%20Door
  ;[0 0.06246 1] Door Control
  ;;[1 1 1] Door Open
  (if (Variables|Default|GetClosed)
    (Transformation|AddActorLocalRotation (* (Math|Rotator|MakeRotator 0.0 0.0 9e+01) -1.0) false false)
    (Variables|Default|SetClosed false)
    (Rendering|Components|TextRender|SetText (Variables|Default|GetDoorReq) (Utilities|Text|ToText(String) " "))))

(event Custom|Close%20Door
  ;[0 0.06246 1] Door Control
  ;;[1 1 1] Door Close
  (if (not (Variables|Default|GetClosed))
    (Transformation|AddActorLocalRotation (* (Math|Rotator|MakeRotator 0.0 0.0 9e+01) 1.0) false false)
    (Variables|Default|SetClosed true)
    (Development|PrintString "Close Door")))

(event Custom|CheckPlayerDistance
  ;[0 0.06246 1] Door Control
  ;;[1 1 1] Door Close
  ;;;[1 1 1] Player Distance Checker
  (if (> (Math|Vector|Distance(Vector) (Transformation|GetActorLocation (Game|GetPlayerCharacter 0)) (Transformation|GetActorLocation)) (Variables|Default|GetPlayerDistance))
    (CallFunction|CloseDoor)))

(event EventBeginPlay
  ;[1 1 1] Start
  (Variables|Default|SetClosed true)
  (Variables|Default|SetPlayerDistance 5e+02)
  (CallFunction|SetRequirementText))

(event Collision|EventActorBeginOverlap
  (params (OtherActor :type Actor%20Object%20Reference))
  ;[1 1 1] Overlap
  (if (Actor|ActorHasTag OtherActor "Player")
    (CallFunction|OpenDoor)))

(event EventTick
  (params (DeltaSeconds :type Float%20%28single-precision%29))
  ;[1 1 1] Update
  (if (not (Variables|Default|GetClosed))
    (CallFunction|CheckPlayerDistance)))

(fn ConstructionScript)

(fn SetRequirementText
  (Rendering|Components|TextRender|SetText (Variables|Default|GetDoorReq) (Utilities|Text|ToText(String) (Variables|Default|GetRequirementText))))