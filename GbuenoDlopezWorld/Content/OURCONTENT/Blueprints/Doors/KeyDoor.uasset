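; KeyDoor is a child door Blueprint that only lets the player trigger it while they hold the key.
; On BeginPlay it sets its requirement text to say a key is needed.
; On overlap by a Player-tagged FPS_Character, it runs the parent overlap logic if GotTheKey is true, otherwise it prints a reminder message.
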(event EventBeginPlay
  (|CallParentFunction)
  (Variables|Default|SetRequirementText "You need the Key!")
  (CallFunction|SetRequirementText))

(event Collision|EventActorBeginOverlap
  (params (OtherActor :type Actor%20Object%20Reference))
  (if (Actor|ActorHasTag OtherActor "Player")
    (bind _asfps_character (Utilities|Casting|CastToFPS_Character OtherActor))
    (if (Variables|/Game/OURCONTENT/FPS/Character/FPS_Character.FPS_Character_C|GetGotTheKey _asfps_character)
      (|CallParentFunction OtherActor)
      (else
        (Development|PrintString "You need The KEY!")))))

(event EventTick
  (params (DeltaSeconds :type Float%20%28single-precision%29))
  (|CallParentFunction DeltaSeconds) ; This node is disabled and will not be called.\nDrag off pins to build functionality.
)

(fn ConstructionScript
  (|CallParentFunction))